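; Blast variant of a radius attack actor that adds a visual effect and sound when its attack zone spawns.
; SpawnAttackZone runs the parent logic, then attaches the Attack Niagara system to the root and plays AttackSfx at the actor's location.
; The actor destroys itself when the effect's finished event fires, or after a short delay if no valid effect is set.
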(event `self.SpawnAttackZone`
  (`parent.SpawnAttackZone`)
  (`self.ShowAttackEffect`)
  (`self.PlayAttackSfx`))

(event `PlayAttackSfx`
  (`GameplayStatics.PlaySoundAtLocation` (`self.AttackSfx`) (`self.K2_GetActorLocation`) (struct) 1.0 1.0 0.0 null null null null))

(event `ShowAttackEffect`
  (bind _attack (`self.Attack`)
    (:`then`
      (bind _returnvalue (`NiagaraFunctionLibrary.SpawnSystemAttached` _attack (`self.DefaultSceneRoot`) "None" (0.0 0.0 0.0) (struct) "KeepRelativeOffset"))
      (add `NiagaraComponent.OnSystemFinished` _returnvalue (delegate `SystemFinished`)))
    (:`else`
      (`KismetSystemLibrary.Delay` 1.0)
      (`self.K2_DestroyActor`))))

(event `SystemFinished`
  (params (PSystem :type "NiagaraComponent Object Reference"))
  (`self.K2_DestroyActor`))

(fn `UserConstructionScript`
  (`parent.UserConstructionScript`))