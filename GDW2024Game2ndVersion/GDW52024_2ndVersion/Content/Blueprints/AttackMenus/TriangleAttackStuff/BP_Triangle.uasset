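; BP_Triangle is a short-lived attack actor, apparently the fire-themed triangle attack.
; On BeginPlay it plays the Fire_attack sound, then destroys itself after a fixed delay.
; Any overlapping actor other than player 0's BP_Player takes damage, and Enemy_AI characters are also launched upward with velocity added to their current motion.
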(event `self.ReceiveBeginPlay`
  (`GameplayStatics.PlaySound2D` "/Game/Blueprints/AttackMenus/TriangleAttackStuff/Fire_attack.Fire_attack" 1.0 1.0 0.0 null null)
  (`KismetSystemLibrary.Delay` 3.0)
  (`self.K2_DestroyActor`))

(event `self.ReceiveActorBeginOverlap`
  (params (OtherActor :type "Actor Object Reference"))
  (bind _asbp_player (cast `/Game/Blueprints/BP_Player` (`GameplayStatics.GetPlayerCharacter` 0)))
  (if (!= OtherActor _asbp_player)
    (`GameplayStatics.ApplyDamage` OtherActor 1.0)
    (bind _asenemy_ai (cast `/Game/Blueprints/Enemies/Enemy_AI` OtherActor))
    (if (== OtherActor _asenemy_ai)
      (`Character.LaunchCharacter` _asenemy_ai (0.0 0.0 500.0) false false))))

(fn `UserConstructionScript`)