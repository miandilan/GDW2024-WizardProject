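; RadiusAttackBase is an area attack actor that damages and reports what lies within a sphere around it.
; TriggerEffect runs SpawnAttackZone, which finds overlapping Pawns, optionally excluding the instigator, and applies radial damage that ignores "Player"-tagged actors.
; Each overlapped actor is broadcast through IceOverlapActor and printed.
; The delayed self-destroy sits inside that loop, so it only runs when something overlaps; a debug sphere is optional.
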(event `self.ReceiveBeginPlay`)

(event `TriggerEffect`
  (`self.SpawnAttackZone`))

(event `SpawnAttackZone`
  (if (`self.drawDebugSphere`)
    (`KismetSystemLibrary.DrawDebugSphere` (`self.K2_GetActorLocation`) (`self.Sphere Radius`) 12 (struct :`G` 0.993655 :`B` 1.0 :`A` 1.0) 2.0 1.0))
  (bind _outactors (`KismetSystemLibrary.SphereOverlapActors` (`self.K2_GetActorLocation`) (`self.Sphere Radius`) (`|MakeArray` "ObjectTypeQuery3" :!type "EObjectTypeQuery Enum") null (select `bool` (`self.ignoreInstigator`) :`true` (`|MakeArray` (`self.GetInstigator`) :!type "Actor Object Reference"))))
  (bind _outactors_2 (`GameplayStatics.GetAllActorsWithTag` "Player"))
  (`GameplayStatics.ApplyRadialDamage` 2.0 (`self.K2_GetActorLocation`) (`self.Sphere Radius`) null _outactors_2 null null)
  (for _array_element _outactors
    (`self.IceOverlapActor` _array_element)
    (`KismetSystemLibrary.PrintString` (`KismetSystemLibrary.GetDisplayName` _array_element))
    (`KismetSystemLibrary.Delay` 2.0)
    (`self.K2_DestroyActor`)))

(fn `UserConstructionScript`)