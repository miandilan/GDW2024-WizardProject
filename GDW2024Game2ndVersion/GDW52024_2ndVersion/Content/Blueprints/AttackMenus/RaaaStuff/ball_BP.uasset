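; Thrown ball projectile Blueprint from the Raaa attack set that damages what it hits.
; On spawn it plays a throw sound and destroys itself after four seconds.
; A Sphere component hit on any actor other than the player character applies one point of damage, plays a hit sound and destroys the ball.
; Debug strings print when it expires or hits.
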(event `self.ReceiveBeginPlay`
  (`GameplayStatics.PlaySound2D` "/Game/Blueprints/AttackMenus/RaaaStuff/RaaaThrow.RaaaThrow" 1.0 1.0 0.0 null null)
  (`KismetSystemLibrary.Delay` 4.0)
  (`self.K2_DestroyActor`)
  (`KismetSystemLibrary.PrintString` "bulletded"))

(event `self.Sphere.OnComponentHit`
  (params (HitComponent :type "PrimitiveComponent Object Reference") (OtherActor :type "Actor Object Reference") (OtherComp :type "PrimitiveComponent Object Reference") (NormalImpulse :type "Vector Structure") (Hit :type "HitResult Structure (by ref)"))
  (bind _asbp_player (cast `/Game/Blueprints/BP_Player` (`GameplayStatics.GetPlayerCharacter` 0)))
  (if (!= OtherActor _asbp_player)
    (`GameplayStatics.ApplyDamage` OtherActor 1.0)
    (`GameplayStatics.PlaySound2D` "/Game/Blueprints/AttackMenus/RaaaStuff/RaaaHit.RaaaHit" 1.0 1.0 0.0 null null)
    (`self.K2_DestroyActor`)
    (`KismetSystemLibrary.PrintString` "Ouch")))

(fn `UserConstructionScript`)