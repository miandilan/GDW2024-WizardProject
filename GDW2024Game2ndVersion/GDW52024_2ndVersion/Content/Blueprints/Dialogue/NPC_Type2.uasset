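; NPC_Type2 is an NPC Blueprint that steps through lines of dialogue on screen, one per Communicate event.
; Each call increments SpeechIndex, lazily creates a UI_Dialogue widget for the first player controller, and writes the current Dialogue array entry into its Speech text.
; Once the index runs past the array, the widget is removed from its parent; the index is never reset here.
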(event `/Game/Blueprints/Dialogue/BPI_Dialogue.Communicate`
  (`/Engine/EditorBlueprintResources/StandardMacros.IncrementInt` (`self.speechIndex`)
    (:`  `
      (if (< (`self.speechIndex`) (`KismetArrayLibrary.Array_Length` (`self.Dialogue`)))
        (`self.ui_Dialogue`
          (:`then`
            _)
          (:`else`
            (bind _returnvalue (`|CreateWidget` "/Game/Blueprints/Dialogue/UI_Dialogue.UI_Dialogue_C" (`GameplayStatics.GetPlayerController` 0)))
            (bind _output_get (set `self.ui_Dialogue` _returnvalue))
            (`UserWidget.AddToViewport` _output_get 0)))
        (`TextBlock.SetText` (`/Game/Blueprints/Dialogue/UI_Dialogue.Speech` (`self.ui_Dialogue`)) (`KismetTextLibrary.Conv_StringToText` (`|GetArrayItem` (`self.Dialogue`) (`self.speechIndex`))))
        (else
          (`Widget.RemoveFromParent` (`self.ui_Dialogue`)))))))

(fn `UserConstructionScript`)