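; Base Blueprint for an advanced enemy that chases the player and makes melee attacks.
; BeginPlay starts a chase loop: AI MoveTo the player, attack on arrival, then repeat after a short delay; failed moves are not retried.
; Attacks start a montage and, if CanHurt is set, immediately sphere-trace forward for pawns, damaging a hit BP_Player.
; RotateAroundPlayer is an empty stub.
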(event `self.ReceiveBeginPlay`
  (`self.ChasePlayer`))

(event `ChasePlayer`
  (`|AIMoveTo` self (0.0 0.0 0.0) (`GameplayStatics.GetPlayerCharacter` 0) 100.0
    (:`OnSuccess`
      (`self.AttackPlayer`)
      (`KismetSystemLibrary.Delay` 2.0)
      (`self.ChasePlayer`))))

(event `RotateAroundPlayer`)

(event `AttackPlayer`
  (bind _returnvalue (`self.K2_GetActorLocation`))
  (`|PlayMontage` (`self.Mesh`)
    (:`then`
      (if (`self.canHurt`)
        (bind (_outhit _returnvalue_2) (`KismetSystemLibrary.SphereTraceSingleForObjects` _returnvalue (+ _returnvalue (* (`KismetMathLibrary.GetForwardVector` (`self.K2_GetActorRotation`)) 250.0)) 50.0 (`|MakeArray` "ObjectTypeQuery3" :!type "EObjectTypeQuery Enum")))
        (if _returnvalue_2
          (bind _asbp_player (cast `/Game/Blueprints/BP_Player` (`.HitActor` (`GameplayStatics.BreakHitResult` _outhit))))
          (`GameplayStatics.ApplyDamage` _asbp_player 1.0))))))

(fn `UserConstructionScript`)