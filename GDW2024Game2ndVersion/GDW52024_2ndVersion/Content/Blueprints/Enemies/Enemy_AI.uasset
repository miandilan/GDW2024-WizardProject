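; Enemy character that spots the player, deals sphere-trace melee damage and shows its health on a widget bar.
; PawnSensing sets a blackboard flag on the AI controller.
; Any hit while health remains sets the player's WallopHit, so the enemy always ragdolls upward and is destroyed after three seconds.
; Only hits at zero health reach the loot branch, whose random pick between upgrade pickups always yields HealthUpgrade.
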(event `DropLoot`
  (bind _returnvalue (`self.K2_GetActorLocation`))
  ;[1 1 1] LootDropSystem
  (bind _outhit (`KismetSystemLibrary.LineTraceSingle` _returnvalue (- _returnvalue (0.0 0.0 200.0)) "TraceTypeQuery1" false (`|MakeArray` (`GameplayStatics.GetPlayerCharacter` 0) :!type "Actor Object Reference")))
  (`|SpawnActorFromClass` (select `int` (`KismetMathLibrary.RandomInteger` 1) :`0` "/Game/Blueprints/Interactables/HealthUpgrade.HealthUpgrade_C" :`1` "/Game/Blueprints/Interactables/DamageUpgrade.DamageUpgrade_C" :!type "Actor Class Reference") (`KismetMathLibrary.MakeTransform` (`NavigationSystemV1.K2_GetRandomReachablePointInRadius` (`.Location` (`GameplayStatics.BreakHitResult` _outhit)) 200.0 null null) (`KismetMathLibrary.MakeRotator` 0.0 0.0 (`KismetMathLibrary.RandomFloatInRange` 0.0 360.0))) "Undefined" "MultiplyWithRoot" null null))

(event `self.ReceiveAnyDamage`
  (params (Damage :type "Float (single-precision)") (DamageType :type "DamageType Object Reference") (InstigatedBy :type "Controller Object Reference") (DamageCauser :type "Actor Object Reference"))
  (bind _mesh (`self.Mesh`))
  ;[1 1 1] Get Damaged and Die
  (if (> (`self.Health`) 0.0)
    (set `self.Health` (- (`self.Health`) Damage))
    (`self.UpdateHealthBar`)
    (bind _asbp_player (cast `/Game/Blueprints/BP_Player` (`GameplayStatics.GetPlayerCharacter` 0)))
    (bind _output_get (set `/Game/Blueprints/BP_Player.WallopHit` true _asbp_player))
    (if _output_get
      (`PrimitiveComponent.SetSimulatePhysics` _mesh true)
      (`PrimitiveComponent.AddImpulse` _mesh (0.0 2500.0 100000.0) "None" false)
      (`GameplayStatics.PlaySound2D` "/Game/Blueprints/Enemies/EnemyDeath_2_0.EnemyDeath_2_0" 1.0 1.0 0.0 null null)
      (`KismetSystemLibrary.Delay` 3.0)
      (`self.K2_DestroyActor`))
    (else
      (for _ (range (+ (`KismetMathLibrary.RandomInteger` 4) 1))
        (`self.DropLoot`))
      (`self.K2_DestroyActor`)
      (`GameplayStatics.PlaySound2D` "/Game/Blueprints/Enemies/EnemyDeath_2_0.EnemyDeath_2_0" 1.0 1.0 0.0 null null))))

(event `Attack Player`
  (bind _returnvalue (`self.K2_GetActorLocation`))
  ;[1 1 1] Damage Player
  (bind (_outhit _returnvalue_2) (`KismetSystemLibrary.SphereTraceSingleForObjects` _returnvalue (+ _returnvalue (* (`KismetMathLibrary.GetForwardVector` (`self.K2_GetActorRotation`)) 250.0)) 50.0 (`|MakeArray` "ObjectTypeQuery3" :!type "EObjectTypeQuery Enum")))
  (if _returnvalue_2
    (bind _asbp_player (cast `/Game/Blueprints/BP_Player` (`.HitActor` (`GameplayStatics.BreakHitResult` _outhit))))
    (`GameplayStatics.ApplyDamage` _asbp_player 20.0)))

(event `self.PawnSensing.OnSeePawn`
  (params (Pawn :type "Pawn Object Reference"))
  ;[1 1 1] Sense Player
  (cast `/Game/Blueprints/BP_Player` Pawn)
  (`BlackboardComponent.SetValueAsBool` (`AIBlueprintHelperLibrary.GetBlackboard` (`AIBlueprintHelperLibrary.GetAIController` self)) "isPlayerSeen?" true))

(event `self.ReceiveBeginPlay`
  ;[1 1 1] HealthBar
  (`self.UpdateHealthBar`))

(fn `UpdateHealthBar`
  (bind _asenemy_health_bar (cast `/Game/Blueprints/Enemies/Enemy_HealthBar` (`WidgetComponent.GetUserWidgetObject` (`self.HealthBar`))))
  (set `/Game/Blueprints/Enemies/Enemy_HealthBar.Health` (`self.Health`) _asenemy_health_bar)
  (return))

(fn `UserConstructionScript`)